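; BP_Cube is an actor set up as a damage source against a BP_Enemy_Melee2 enemy, but its damage logic is currently unwired.
; On BeginPlay it casts its Class variable, finds an actor of that class and caches it as EnemyRef.
; The DamageCollider overlap event is empty.
; A disconnected branch would apply CubeDamage and print a debug message when EnemyRef is within a fixed distance.
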(event `self.ReceiveBeginPlay`
  (bind _asbp_enemy_melee_2 (castclass `/Game/Enemy/EnemyMelee/BP_Enemy_Melee2` (`self.Class`)))
  (bind _returnvalue (`GameplayStatics.GetActorOfClass` _asbp_enemy_melee_2))
  (bind _asbp_enemy_melee_2_2 (cast `/Game/Enemy/EnemyMelee/BP_Enemy_Melee2` _returnvalue))
  (set `self.EnemyRef` _asbp_enemy_melee_2_2))

(event `self.DamageCollider.OnComponentBeginOverlap`
  (params (OverlappedComponent :type "PrimitiveComponent Object Reference") (OtherActor :type "Actor Object Reference") (OtherComp :type "PrimitiveComponent Object Reference") (OtherBodyIndex :type Integer) (bFromSweep :type Boolean) (SweepResult :type "HitResult Structure (by ref)")))

(fn `UserConstructionScript`)