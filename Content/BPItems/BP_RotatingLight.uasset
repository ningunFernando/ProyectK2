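; BP_RotatingLight is a red alarm beacon whose lights spin and sound off while triggered by a box volume.
; Box begin and end overlap set and clear a trigger flag, with no filter on the overlapping actor.
; While the flag is set, Tick yaws two components by a delta-time-scaled speed and starts a new Camera_Shutter sound at the beacon mesh every frame.
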(event `self.ReceiveTick`
  (params (DeltaSeconds :type "Float (single-precision)"))
  (if (`self.IstRIGERED`)
    (`self.PlaySound`)))

(event `self.Box.OnComponentBeginOverlap`
  (params (OverlappedComponent :type "PrimitiveComponent Object Reference") (OtherActor :type "Actor Object Reference") (OtherComp :type "PrimitiveComponent Object Reference") (OtherBodyIndex :type Integer) (bFromSweep :type Boolean) (SweepResult :type "HitResult Structure (by ref)"))
  (set `self.IstRIGERED` true))

(event `PlaySound`
  (`SceneComponent.K2_AddLocalRotation` (`self.02`) (* (`KismetMathLibrary.MakeRotator` 0.0 0.0 (`self.LightRotationSpeed`)) (stale `self.ReceiveTick` DeltaSeconds)) false false)
  (`SceneComponent.K2_AddLocalRotation` (`self.01`) (* (`KismetMathLibrary.MakeRotator` 0.0 0.0 (`self.LightRotationSpeed`)) (stale `self.ReceiveTick` DeltaSeconds)) false false)
  (`GameplayStatics.PlaySoundAtLocation` "/Engine/VREditor/Sounds/UI/Camera_Shutter.Camera_Shutter" (`SceneComponent.K2_GetComponentLocation` (`self.Bec-Alarma-Rosu-High-Poly`)) (struct) 1.0 1.0 0.0 null null null null))

(event `self.Box.OnComponentEndOverlap`
  (params (OverlappedComponent :type "PrimitiveComponent Object Reference") (OtherActor :type "Actor Object Reference") (OtherComp :type "PrimitiveComponent Object Reference") (OtherBodyIndex :type Integer))
  (set `self.IstRIGERED` false))

(fn `UserConstructionScript`)