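; Enemy character Blueprint that can be launched in the direction the player is looking.
; BeginPlay caches the first-person player character, and the Launch event throws the enemy along that character's camera forward vector, overriding its current velocity.
; Sphere overlap events toggle and print the player's IsEnemy flag on enter and exit, though an author comment marks them as non-working leftovers.
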(event `self.ReceiveBeginPlay`
  ;[0.1195 0.6376 1] Crear una variable con la referencia
  (bind _asbp_first_person_character (cast `/Game/FirstPerson/Blueprints/BP_FirstPersonCharacter` (`GameplayStatics.GetPlayerCharacter` 0)))
  (set `self.PlayerRef` _asbp_first_person_character))

(event `/Game/Extras/BPI_TK.Launch`
  ;[0.1195 0.6376 1] Lanzar Enemigo
  (`self.LaunchCharacter` (* (`SceneComponent.GetForwardVector` (`/Game/FirstPerson/Blueprints/BP_FirstPersonCharacter.FirstPersonCamera` (`self.PlayerRef`))) 10000.0) true true))

(event `self.Sphere.OnComponentBeginOverlap`
  (params (OverlappedComponent :type "PrimitiveComponent Object Reference") (OtherActor :type "Actor Object Reference") (OtherComp :type "PrimitiveComponent Object Reference") (OtherBodyIndex :type Integer) (bFromSweep :type Boolean) (SweepResult :type "HitResult Structure (by ref)"))
  ;[1 0 0] No sirven, pero igual lo dejo por si las dudas
  (bind _asbp_first_person_character (cast `/Game/FirstPerson/Blueprints/BP_FirstPersonCharacter` OtherActor))
  (bind _output_get (set `/Game/FirstPerson/Blueprints/BP_FirstPersonCharacter.IsEnemy` true _asbp_first_person_character))
  (`KismetSystemLibrary.PrintString` (`KismetStringLibrary.Conv_BoolToString` _output_get)))

(event `self.Sphere.OnComponentEndOverlap`
  (params (OverlappedComponent :type "PrimitiveComponent Object Reference") (OtherActor :type "Actor Object Reference") (OtherComp :type "PrimitiveComponent Object Reference") (OtherBodyIndex :type Integer))
  ;[1 0 0] No sirven, pero igual lo dejo por si las dudas
  (bind _asbp_first_person_character (cast `/Game/FirstPerson/Blueprints/BP_FirstPersonCharacter` OtherActor))
  (bind _output_get (set `/Game/FirstPerson/Blueprints/BP_FirstPersonCharacter.IsEnemy` false _asbp_first_person_character))
  (`KismetSystemLibrary.PrintString` (`KismetStringLibrary.Conv_BoolToString` _output_get)))

(fn `UserConstructionScript`)