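; Melee enemy character that chases the player and deals damage up close.
; Pawn sensing triggers an AI move to the player, playing an attack montage on arrival behind a brief CanAttack lockout; Tick stops movement while the player is unseen.
; Separately, attack-collider overlap starts a looping timer, cleared on exit, that applies melee damage when CanAttack is set and the player is within range, with debug prints.
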(event `self.PawnSensing.OnSeePawn`
  (params (Pawn :type "Pawn Object Reference"))
  ;[1 0 0] Seguir al jugador
  (set `self.isSeeingPlayer` true)
  (`self.FollowPlayer`))

(event `FollowPlayer`
  ;[1 0 0] Logica para seguir al jugador
  (if (`self.isSeeingPlayer`)
    (`|AIMoveTo` self (0.0 0.0 0.0) (`self.PlayerRef`) 70.0 true
      (:`OnSuccess`
        (if (`self.CanAttack`)
          (set `self.CanAttack` false)
          (`self.PlayAnimMontage` "/Game/Enemy/EnemyMelee/Animate/AM_EnemyMelee.AM_EnemyMelee")
          (`KismetSystemLibrary.Delay` 0.2)
          (set `self.CanAttack` true))))
    (else
      (set `self.isSeeingPlayer` false))))

(event `self.ReceiveTick`
  (params (DeltaSeconds :type "Float (single-precision)"))
  ;[1 0 0] Se detenga si lo ve (aun no estoy testeando)
  (if (not (`self.isSeeingPlayer`))
    (`NavMovementComponent.StopActiveMovement` (`self.CharacterMovement`))))

(event `self.ColliderAttack.OnComponentBeginOverlap`
  (params (OverlappedComponent :type "PrimitiveComponent Object Reference") (OtherActor :type "Actor Object Reference") (OtherComp :type "PrimitiveComponent Object Reference") (OtherBodyIndex :type Integer) (bFromSweep :type Boolean) (SweepResult :type "HitResult Structure (by ref)"))
  ;[1 0 0] Hacer daño
  (bind _returnvalue (`KismetSystemLibrary.K2_SetTimerDelegate` (delegate `hacerDanio`) 1.0 true)))

(event `self.ColliderAttack.OnComponentEndOverlap`
  (params (OverlappedComponent :type "PrimitiveComponent Object Reference") (OtherActor :type "Actor Object Reference") (OtherComp :type "PrimitiveComponent Object Reference") (OtherBodyIndex :type Integer))
  ;[1 0 0] Hacer daño
  (`KismetSystemLibrary.K2_ClearAndInvalidateTimerHandle` (stale `self.ColliderAttack.OnComponentBeginOverlap` _returnvalue)))

(event `hacerDanio`
  (bind _returnvalue (< (`KismetMathLibrary.Vector_Distance` (`self.K2_GetActorLocation` (`self.PlayerRef`)) (`self.K2_GetActorLocation` self)) 200.0))
  ;[1 0 0] Hacer daño
  (if (`self.CanAttack`)
    (`KismetSystemLibrary.PrintString` "Hello" _returnvalue true (struct :`R` 0.282014 :`G` 1.0 :`A` 1.0))
    (if _returnvalue
      (bind _output_get (set `self.DamageEnemy` (`self.DamageMelee`)))
      (`GameplayStatics.ApplyDamage` (`self.PlayerRef`) _output_get null self)
      (`KismetSystemLibrary.PrintString` "Hizo Daño" true true (struct :`R` 1.0 :`B` 0.014578 :`A` 1.0) 5.0))))

(fn `UserConstructionScript`
  (`parent.UserConstructionScript`))