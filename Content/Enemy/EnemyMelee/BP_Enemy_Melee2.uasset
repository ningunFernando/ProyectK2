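; Melee enemy character that chases the player once PawnSensing spots them, playing a hook punch montage on reaching them.
; An attack collider starts a looping timer that damages the player when attacking is allowed and in range.
; Overlaps on its hurt collider near the player apply dash damage and knockback; any damage lowers clamped health, destroying it at zero.
; Tick updates the health bar's fill and rotation.
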(event `self.ReceiveBeginPlay`
  (`parent.ReceiveBeginPlay`))

(event `self.PawnSensing.OnSeePawn`
  (params (Pawn :type "Pawn Object Reference"))
  ;[1 0 0] Seguir al jugador
  (set `self.isSeeingPlayer` true)
  (`self.FollowPlayer`))

(event `FollowPlayer`
  ;[1 0 0] Logica para seguir al jugador
  (if (`self.isSeeingPlayer`)
    (`|AIMoveTo` self (0.0 0.0 0.0) (`self.PlayerRef`) 70.0 true
      (:`OnSuccess`
        (if (`self.CanAttack`)
          (set `self.CanAttack` false)
          (bind _returnvalue (`self.PlayAnimMontage` "/Game/Enemy/EnemyMelee/Animate/Hook_Punch_Anim_Montage.Hook_Punch_Anim_Montage"))
          (bind _returnvalue_2 (* _returnvalue 0.4))
          (`KismetSystemLibrary.Delay` _returnvalue_2)
          (set `self.CanAttack` true)
          (`KismetSystemLibrary.Delay` _returnvalue_2))))
    (else
      (set `self.isSeeingPlayer` false)
      (`KismetSystemLibrary.PrintString` "ya no lo ve" true true (struct :`R` 0.115871 :`G` 0.181282 :`B` 1.0 :`A` 1.0) 5.0))))

(event `self.ReceiveTick`
  (params (DeltaSeconds :type "Float (single-precision)"))
  (bind _barravidaenemy (`self.BarraVidaEnemy`))
  (bind _barravidaenemy_2 (`self.BarraVidaEnemy`))
  ;[1 0.9216 0] Barra de vida
  (`ProgressBar.SetPercent` (`/Game/Enemy/UI_Enemy/WP_BarraEnemy.EnemyBar` (`self.BarraRef`)) (/ (`self.Healt`) 50.0))
  (if (`self.isSeeingPlayer`)
    (`SceneComponent.K2_SetWorldRotation` _barravidaenemy (`KismetMathLibrary.FindLookAtRotation` (`SceneComponent.K2_GetComponentLocation` _barravidaenemy) (`SceneComponent.K2_GetComponentLocation` (`self.ColliderAttack`))) false false)
    (else
      (`SceneComponent.K2_SetWorldRotation` _barravidaenemy_2 (`KismetMathLibrary.FindLookAtRotation` (`SceneComponent.K2_GetComponentLocation` _barravidaenemy_2) (`SceneComponent.K2_GetComponentLocation` (`Actor.RootComponent` (`GameplayStatics.GetPlayerCameraManager` 0)))) false false)))
  ;[1 0 0] Seguir al jugador
  (if (not (`self.isSeeingPlayer`))
    (`NavMovementComponent.StopActiveMovement` (`self.CharacterMovement`))))

(event `self.ColliderAttack.OnComponentBeginOverlap`
  (params (OverlappedComponent :type "PrimitiveComponent Object Reference") (OtherActor :type "Actor Object Reference") (OtherComp :type "PrimitiveComponent Object Reference") (OtherBodyIndex :type Integer) (bFromSweep :type Boolean) (SweepResult :type "HitResult Structure (by ref)"))
  ;[1 0 0] Hacer daño
  (bind _returnvalue (`KismetSystemLibrary.K2_SetTimerDelegate` (delegate `hacerDanio`) 1.0 true)))

(event `self.ColliderAttack.OnComponentEndOverlap`
  (params (OverlappedComponent :type "PrimitiveComponent Object Reference") (OtherActor :type "Actor Object Reference") (OtherComp :type "PrimitiveComponent Object Reference") (OtherBodyIndex :type Integer))
  ;[1 0 0] Hacer daño
  (`KismetSystemLibrary.K2_ClearAndInvalidateTimerHandle` (stale `self.ColliderAttack.OnComponentBeginOverlap` _returnvalue)))

(event `hacerDanio`
  ;[1 0 0] Hacer daño
  (if (`self.CanAttack`)
    (if (< (`KismetMathLibrary.Vector_Distance` (`self.K2_GetActorLocation` (`self.PlayerRef`)) (`self.K2_GetActorLocation` self)) 150.0)
      (bind _output_get (set `self.DamageEnemy` (`self.DamageMelee`)))
      (`GameplayStatics.ApplyDamage` (`self.PlayerRef`) _output_get null self))))

(event `self.RecibeDanio.OnComponentBeginOverlap`
  (params (OverlappedComponent :type "PrimitiveComponent Object Reference") (OtherActor :type "Actor Object Reference") (OtherComp :type "PrimitiveComponent Object Reference") (OtherBodyIndex :type Integer) (bFromSweep :type Boolean) (SweepResult :type "HitResult Structure (by ref)"))
  (bind _healt (`self.Healt`))
  ;[1 0.927 0] sistema para recibir damio del jugador
  (if (`KismetMathLibrary.Conv_IntToBool` (`KismetMathLibrary.And_IntInt` (`KismetMathLibrary.Conv_BoolToInt` (> (`self.Healt`) 0.0)) (`KismetMathLibrary.Conv_BoolToInt` (< (`KismetMathLibrary.Vector_Distance` (`self.K2_GetActorLocation` (`self.PlayerRef`)) (`self.K2_GetActorLocation` self)) 130.0))))
    (`GameplayStatics.ApplyDamage` self (`self.DashPlayerDamage`) null (`self.PlayerRef`))
    (`self.LaunchCharacter` self (500.0 100.0 500.0) true true)
    (if (<= _healt 0.0)
      (`self.K2_DestroyActor`)
      (`KismetSystemLibrary.PrintString` (`KismetStringLibrary.Conv_DoubleToString` _healt) true true (struct :`R` 1.0 :`G` 0.700821 :`A` 1.0) 5.0)
      (`KismetSystemLibrary.PrintString` "el jugador" true true (struct :`R` 1.0 :`B` 0.63286 :`A` 1.0) 5.0)
      (else
        (`KismetSystemLibrary.Delay` 2.0)))))

(event `self.ReceiveAnyDamage`
  (params (Damage :type "Float (single-precision)") (DamageType :type "DamageType Object Reference") (InstigatedBy :type "Controller Object Reference") (DamageCauser :type "Actor Object Reference"))
  ;[1 0.9493 0] Recibir danio en general
  (bind _output_get (set `self.Healt` (`KismetMathLibrary.FClamp` (- (`self.Healt`) Damage) 0.0 (`self.MaxHealt`))))
  (`KismetSystemLibrary.PrintString` (`KismetStringLibrary.Conv_DoubleToString` _output_get) true true (struct :`R` 1.0 :`G` 0.506319 :`A` 1.0) 5.0)
  (if (<= (`self.Healt`) 0.0)
    (`self.K2_DestroyActor`)
    (else
      (`KismetSystemLibrary.Delay` 2.0))))

(fn `UserConstructionScript`
  (`parent.UserConstructionScript`))