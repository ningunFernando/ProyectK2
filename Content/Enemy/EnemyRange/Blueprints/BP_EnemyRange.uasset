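; BP_EnemyRange is an enemy Blueprint that detects the first-person player and supplies attack hit checks.
; PawnSensing sets the AI Blackboard's hasSeenPlayer flag on seeing the player, then clears it after a short delay.
; HitDetector sphere-traces at the right forearm socket and applies damage to the player.
; AttackPlayer sphere-traces ahead for the player but does nothing after the cast.
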(event `self.PawnSensing.OnSeePawn`
  (params (Pawn :type "Pawn Object Reference"))
  (bind _returnvalue (`AIBlueprintHelperLibrary.GetBlackboard` (`AIBlueprintHelperLibrary.GetAIController` self)))
  ;[1 1 1] Start chasing character
  (cast `/Game/FirstPerson/Blueprints/BP_FirstPersonCharacter` Pawn)
  (`BlackboardComponent.SetValueAsBool` _returnvalue "hasSeenPlayer" true)
  (`KismetSystemLibrary.Delay` 3.0)
  (`BlackboardComponent.SetValueAsBool` _returnvalue "hasSeenPlayer" false))

(event `AttackPlayer`
  (bind _returnvalue (`self.K2_GetActorLocation`))
  ;[1 1 1] Realizar el ataque
  (bind (_outhit _returnvalue_2) (`KismetSystemLibrary.SphereTraceSingleForObjects` _returnvalue (+ _returnvalue (* (`KismetMathLibrary.GetForwardVector` (`self.K2_GetActorRotation`)) 250.0)) 120.0 (`|MakeArray` "ObjectTypeQuery3" :!type "EObjectTypeQuery Enum")))
  (if _returnvalue_2
    (cast `/Game/FirstPerson/Blueprints/BP_FirstPersonCharacter` (`.HitActor` (`GameplayStatics.BreakHitResult` _outhit)))))

(fn `HitDetector`
  (bind _returnvalue (`SceneComponent.GetSocketLocation` (`self.Mesh`) "lowerarm_r"))
  (bind _outhit (`KismetSystemLibrary.SphereTraceSingleForObjects` _returnvalue _returnvalue 50.0 (`|MakeArray` "ObjectTypeQuery3" :!type "EObjectTypeQuery Enum")))
  (bind _asbp_first_person_character (cast `/Game/FirstPerson/Blueprints/BP_FirstPersonCharacter` (`.HitActor` (`GameplayStatics.BreakHitResult` _outhit))))
  (`GameplayStatics.ApplyDamage` _asbp_first_person_character 1.0))

(fn `UserConstructionScript`)