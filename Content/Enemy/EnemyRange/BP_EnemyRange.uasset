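; Ranged enemy character that spawns a rifle in its hand and pursues the player once PawnSensing spots them.
; AIMoveTo success plays the shooting montage, while a delayed Tick spawns projectiles at close range and applies damage directly, independent of impact.
; Close-range player overlaps damage and launch it; AnyDamage clamps health, destroying enemy and rifle at zero.
; Tick also updates and rotates the health bar.
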(event `self.ReceiveBeginPlay`
  ;[1 0.8855 0] Heredar del padre
  (`parent.ReceiveBeginPlay`)
  ;[0.7339 0 1] Equipar la arma
  (bind _returnvalue (`|SpawnActorFromClass` "/Game/FirstPerson/Blueprints/BP_Pickup_Rifle.BP_Pickup_Rifle_C" (`KismetMathLibrary.MakeTransform` (0.0 0.0 0.0)) "Undefined" "MultiplyWithRoot" null null))
  (bind _output_get (set `self.ArmaEquipable` _returnvalue))
  (`self.K2_AttachToComponent` _output_get (`self.Mesh`) "armaSocket" "KeepRelative" "KeepRelative" "KeepRelative" true))

(event `self.PawnSensing.OnSeePawn`
  (params (Pawn :type "Pawn Object Reference"))
  ;[0 0.9727 1] Seguir al jugador
  (set `self.isSeeingPlayer` true)
  (`self.FollowPlayer`))

(event `FollowPlayer`
  ;[0 1 0.9713] Logica para seguir al jugador y hacer daño
  (if (`self.isSeeingPlayer`)
    (`|AIMoveTo` self (0.0 0.0 0.0) (`self.PlayerRef`) 300.0 true
      (:`OnSuccess`
        (if (`self.CanAttack`)
          (set `self.CanAttack` false)
          (bind _returnvalue (`self.PlayAnimMontage` "/Game/Enemy/EnemyRange/Animation/Shoot_Rifle_Montage.Shoot_Rifle_Montage"))
          (bind _returnvalue_2 (* _returnvalue 0.4))
          (`KismetSystemLibrary.Delay` _returnvalue_2)
          (set `self.CanAttack` true)
          (`KismetSystemLibrary.Delay` _returnvalue_2))))
    (else
      (set `self.isSeeingPlayer` false)
      (`KismetSystemLibrary.PrintString` "Ya no vel al jugador" true true (struct :`R` 0.303794 :`G` 0.133661 :`B` 1.0 :`A` 1.0) 5.0))))

(event `self.ReceiveTick`
  (params (DeltaSeconds :type "Float (single-precision)"))
  (bind _barravidaenemy (`self.BarraVidaEnemy`))
  (bind _barravidaenemy_2 (`self.BarraVidaEnemy`))
  ;[0 1 0.1046] Barra de vida
  (`ProgressBar.SetPercent` (`/Game/Enemy/UI_Enemy/WP_BarraEnemy.EnemyBar` (`self.BarraRef`)) (/ (`self.Healt`) 50.0))
  (if (`self.isSeeingPlayer`)
    (`SceneComponent.K2_SetWorldRotation` _barravidaenemy (`KismetMathLibrary.FindLookAtRotation` (`SceneComponent.K2_GetComponentLocation` _barravidaenemy) (`SceneComponent.K2_GetComponentLocation` (`self.SpawnBall`))) false false)
    (else
      (`SceneComponent.K2_SetWorldRotation` _barravidaenemy_2 (`KismetMathLibrary.FindLookAtRotation` (`SceneComponent.K2_GetComponentLocation` _barravidaenemy_2) (`SceneComponent.K2_GetComponentLocation` (`Actor.RootComponent` (`GameplayStatics.GetPlayerCameraManager` 0)))) false false)))
  ;[0 1 0.9933] Dejar de seguir al jugador
  (if (`self.isSeeingPlayer`)
    ;[0.7264 0 1] Instaciar la bala
    (`KismetSystemLibrary.Delay` 2.0)
    (if (< (`KismetMathLibrary.Vector_Distance` (`self.K2_GetActorLocation` (`self.PlayerRef`)) (`self.K2_GetActorLocation` self)) 400.0)
      (bind _returnvalue (`|SpawnActorFromClass` "/Game/FirstPerson/Blueprints/BP_FirstPersonProjectile.BP_FirstPersonProjectile_C" (`KismetMathLibrary.Conv_VectorToTransform` (`SceneComponent.K2_GetComponentLocation` (`self.SpawnBall`))) "Undefined" "MultiplyWithRoot" null null))
      (`GameplayStatics.ApplyDamage` (`self.PlayerRef`) (`self.BallDamage`) null _returnvalue))
    (else
      (`NavMovementComponent.StopActiveMovement` (`self.CharacterMovement`)))))

(event `self.RecibirDanio.OnComponentBeginOverlap`
  (params (OverlappedComponent :type "PrimitiveComponent Object Reference") (OtherActor :type "Actor Object Reference") (OtherComp :type "PrimitiveComponent Object Reference") (OtherBodyIndex :type Integer) (bFromSweep :type Boolean) (SweepResult :type "HitResult Structure (by ref)"))
  (bind _healt (`self.Healt`))
  ;[1 0 0] Recibir daño de jugador
  (if (`KismetMathLibrary.Conv_IntToBool` (`KismetMathLibrary.And_IntInt` (`KismetMathLibrary.Conv_BoolToInt` (> (`self.Healt`) 0.0)) (`KismetMathLibrary.Conv_BoolToInt` (< (`KismetMathLibrary.Vector_Distance` (`self.K2_GetActorLocation` self) (`self.K2_GetActorLocation` (`self.PlayerRef`))) 130.0))))
    (`GameplayStatics.ApplyDamage` self (`self.DashPlayerDamage`) null (`self.PlayerRef`))
    (`self.LaunchCharacter` self (500.0 100.0 500.0) false false)
    (if (<= _healt 0.0)
      (`self.K2_DestroyActor`)
      (`self.K2_DestroyActor` (`self.ArmaEquipable`))
      (`KismetSystemLibrary.PrintString` (`KismetStringLibrary.Conv_DoubleToString` _healt))
      (`KismetSystemLibrary.PrintString` "El jugador" true true (struct :`R` 1.0 :`B` 0.107647 :`A` 1.0) 5.0)
      (else
        (`KismetSystemLibrary.Delay` 2.0)))))

(event `self.ReceiveAnyDamage`
  (params (Damage :type "Float (single-precision)") (DamageType :type "DamageType Object Reference") (InstigatedBy :type "Controller Object Reference") (DamageCauser :type "Actor Object Reference"))
  ;[1 0.007402 0] Sistema de reibir danio
  (bind _output_get (set `self.Healt` (`KismetMathLibrary.FClamp` (- (`self.Healt`) Damage) 0.0 (`self.MaxHealt`))))
  (`KismetSystemLibrary.PrintString` (`KismetStringLibrary.Conv_DoubleToString` _output_get) true true (struct :`R` 1.0 :`G` 0.656913 :`B` 0.022275 :`A` 1.0) 5.0)
  (if (<= (`self.Healt`) 0.0)
    (`self.K2_DestroyActor`)
    (`self.K2_DestroyActor` (`self.ArmaEquipable`))
    (else
      (`KismetSystemLibrary.Delay` 2.0))))

(fn `UserConstructionScript`
  (`parent.UserConstructionScript`))