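; Boss enemy character that chases and attacks the player, with a world-space health bar updated on Tick.
; Pawn sensing triggers AI movement and an attack montage on arrival, and Tick teleports the boss to the player when too far away.
; A looping timer during attack-collider overlap applies damage if CanAttack and range checks pass.
; Hit-collider overlaps apply damage and knockback based on cube or player proximity, and zero health destroys it.
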(event `self.ReceiveTick`
  (params (DeltaSeconds :type "Float (single-precision)"))
  (bind _barravidaenemy (`self.BarraVidaEnemy`))
  (bind _barravidaenemy_2 (`self.BarraVidaEnemy`))
  (bind _playerref (`self.PlayerRef`))
  ;[0 1 0.2542] Barra de vida
  (`ProgressBar.SetPercent` (`/Game/Enemy/UI_Enemy/WP_BarraEnemy.EnemyBar` (`self.BarraRef`)) (/ (`self.Healt`) 50.0))
  (if (`self.SeePlayer`)
    (`SceneComponent.K2_SetWorldRotation` _barravidaenemy (`KismetMathLibrary.FindLookAtRotation` (`SceneComponent.K2_GetComponentLocation` _barravidaenemy) (`SceneComponent.K2_GetComponentLocation` (`self.ColliderAttack`))) false false)
    (else
      (`SceneComponent.K2_SetWorldRotation` _barravidaenemy_2 (`KismetMathLibrary.FindLookAtRotation` (`SceneComponent.K2_GetComponentLocation` _barravidaenemy_2) (`SceneComponent.K2_GetComponentLocation` (`PlayerCameraManager.TransformComponent` (`GameplayStatics.GetPlayerCameraManager` 0)))) false false)))
  (if (`self.SeePlayer`)
    ;[0.8072 0 1] Hacer TP al jugador
    (if (> (`KismetMathLibrary.Vector_Distance` (`self.K2_GetActorLocation` (`self.PlayerRef`)) (`self.K2_GetActorLocation` self)) 1000.0)
      (bind _output_get (set `self.TP_pos` (`self.GetTransform` _playerref)))
      (`self.K2_SetActorLocationAndRotation` :`self` self :`NewLocation` (`KismetMathLibrary.TransformLocation` _output_get (`KismetMathLibrary.Conv_DoubleToVector` (`SkeletalMeshComponent.GetPosition` (`/Game/FirstPerson/Blueprints/BP_FirstPersonCharacter.FirstPersonMesh` _playerref))))))
    (else
      (`NavMovementComponent.StopActiveMovement` (`self.CharacterMovement`)))))

(event `self.ColliderAttack.OnComponentBeginOverlap`
  (params (OverlappedComponent :type "PrimitiveComponent Object Reference") (OtherActor :type "Actor Object Reference") (OtherComp :type "PrimitiveComponent Object Reference") (OtherBodyIndex :type Integer) (bFromSweep :type Boolean) (SweepResult :type "HitResult Structure (by ref)"))
  ;[1 0 0] Hacer daño
  (bind _returnvalue (`KismetSystemLibrary.K2_SetTimerDelegate` (delegate `HacerDanio`) 1.0 true)))

(event `self.PawnSensing.OnSeePawn`
  (params (Pawn :type "Pawn Object Reference"))
  ;[0 0.8148 1] Ver al jugador
  (set `self.SeePlayer` true)
  (`self.FollowPlayer`))

(event `self.ColliderAttack.OnComponentEndOverlap`
  (params (OverlappedComponent :type "PrimitiveComponent Object Reference") (OtherActor :type "Actor Object Reference") (OtherComp :type "PrimitiveComponent Object Reference") (OtherBodyIndex :type Integer))
  ;[1 0 0] Hacer daño
  (`KismetSystemLibrary.K2_ClearAndInvalidateTimerHandle` (stale `self.ColliderAttack.OnComponentBeginOverlap` _returnvalue)))

(event `FollowPlayer`
  ;[0 0.8148 1] Seguir al jugador
  (if (`self.SeePlayer`)
    (`|AIMoveTo` self (0.0 0.0 0.0) (`self.PlayerRef`) 100.0
      (:`OnSuccess`
        (if (`self.CanAttack`)
          (set `self.CanAttack` false)
          (bind _returnvalue (`self.PlayAnimMontage` "/Game/Enemy/BossEnemy/Animaciones/AM_EnemyBoss.AM_EnemyBoss"))
          (bind _returnvalue_2 (* _returnvalue 0.6))
          (`KismetSystemLibrary.Delay` _returnvalue_2)
          (set `self.CanAttack` true)
          (`KismetSystemLibrary.Delay` _returnvalue_2))))
    (else
      (set `self.SeePlayer` false))))

(event `self.ReceiveAnyDamage`
  (params (Damage :type "Float (single-precision)") (DamageType :type "DamageType Object Reference") (InstigatedBy :type "Controller Object Reference") (DamageCauser :type "Actor Object Reference"))
  ;[0 1 0.2542] Evento de restar vida por daño
  (bind _output_get (set `self.Healt` (`KismetMathLibrary.FClamp` (- (`self.Healt`) Damage) 0.0 (`self.MaxHealt`))))
  (`KismetSystemLibrary.PrintString` (`KismetStringLibrary.Conv_DoubleToString` _output_get) true true (struct :`R` 1.0 :`G` 0.506319 :`A` 1.0) 5.0)
  (if (<= (`self.Healt`) 0.0)
    (`self.K2_DestroyActor`)
    (else
      (`KismetSystemLibrary.Delay` 2.0))))

(event `HacerDanio`
  (bind _canattack (`self.CanAttack`))
  ;[1 0 0] Hacer daño
  (`KismetSystemLibrary.PrintString` (`KismetStringLibrary.Conv_BoolToString` _canattack) true true (struct :`R` 1.0 :`B` 0.262702 :`A` 1.0) 5.0)
  (if _canattack
    (if (< (`KismetMathLibrary.Vector_Distance` (`self.K2_GetActorLocation` (`self.PlayerRef`)) (`self.K2_GetActorLocation` self)) 150.0)
      (`GameplayStatics.ApplyDamage` (`self.PlayerRef`) (`self.DamageBoss`) null self))))

(event `self.ReceiveBeginPlay`
  ;[1 0.9216 0] Referencia al jugador
  (bind _asbp_first_person_character (cast `/Game/FirstPerson/Blueprints/BP_FirstPersonCharacter` (`GameplayStatics.GetPlayerCharacter` 0)))
  (set `self.PlayerRef` _asbp_first_person_character)
  ;[1 0.9216 0] Referencia a la barra de vida
  (bind _aswp_barra_enemy (cast `/Game/Enemy/UI_Enemy/WP_BarraEnemy` (`WidgetComponent.GetWidget` (`self.BarraVidaEnemy`))))
  (set `self.BarraRef` _aswp_barra_enemy)
  ;[0 1 0.2542] Setear la vida
  (set `self.Healt` (`self.MaxHealt`))
  (bind _asbp_cube (castclass `/Game/Extras/BP_Cube` "/Game/Extras/BP_Cube.BP_Cube_C"))
  (bind _returnvalue (`GameplayStatics.GetActorOfClass` _asbp_cube))
  (bind _asbp_cube_2 (cast `/Game/Extras/BP_Cube` _returnvalue))
  (set `self.CubeRef` _asbp_cube_2))

(event `self.RecibirDanio.OnComponentBeginOverlap`
  (params (OverlappedComponent :type "PrimitiveComponent Object Reference") (OtherActor :type "Actor Object Reference") (OtherComp :type "PrimitiveComponent Object Reference") (OtherBodyIndex :type Integer) (bFromSweep :type Boolean) (SweepResult :type "HitResult Structure (by ref)"))
  (bind _healt (`self.Healt`))
  (bind _healt_2 (`self.Healt`))
  (bind _returnvalue (`self.K2_GetActorLocation` self))
  (bind _returnvalue_2 (> (`self.Healt`) 0.0))
  ;[1 0 0] Recibir daño
  (if (`KismetMathLibrary.Conv_IntToBool` (`KismetMathLibrary.And_IntInt` (`KismetMathLibrary.Conv_BoolToInt` (< (`KismetMathLibrary.Vector_Distance` _returnvalue (`self.K2_GetActorLocation` (`self.CubeRef`))) 400.0)) (`KismetMathLibrary.Conv_BoolToInt` _returnvalue_2)))
    (`GameplayStatics.ApplyDamage` self 20.0 null (`self.CubeRef`))
    (`self.LaunchCharacter` self (500.0 100.0 500.0) true true)
    (if (<= _healt_2 0.0)
      (`self.K2_DestroyActor`)
      (`KismetSystemLibrary.PrintString` (`KismetStringLibrary.Conv_DoubleToString` _healt_2) true true (struct :`R` 1.0 :`G` 0.700821 :`A` 1.0) 5.0)
      (`KismetSystemLibrary.PrintString` "el cubo" true true (struct :`R` 1.0 :`B` 0.63286 :`A` 1.0) 5.0)
      (else
        (`KismetSystemLibrary.Delay` 2.0)))
    (elif (`KismetMathLibrary.Conv_IntToBool` (`KismetMathLibrary.And_IntInt` (`KismetMathLibrary.Conv_BoolToInt` _returnvalue_2) (`KismetMathLibrary.Conv_BoolToInt` (< (`KismetMathLibrary.Vector_Distance` (`self.K2_GetActorLocation` (`self.PlayerRef`)) _returnvalue) 130.0))))
      (`GameplayStatics.ApplyDamage` self 30.0 null (`self.PlayerRef`))
      (`self.LaunchCharacter` self (500.0 100.0 500.0) true true)
      (if (<= _healt 0.0)
        (`self.K2_DestroyActor`)
        (`KismetSystemLibrary.PrintString` (`KismetStringLibrary.Conv_DoubleToString` _healt) true true (struct :`R` 1.0 :`G` 0.700821 :`A` 1.0) 5.0)
        (`KismetSystemLibrary.PrintString` "el jugador" true true (struct :`R` 1.0 :`B` 0.63286 :`A` 1.0) 5.0)
        (else
          (`KismetSystemLibrary.Delay` 2.0))))))

(fn `UserConstructionScript`)